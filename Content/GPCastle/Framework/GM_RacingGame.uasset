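; Game mode for a timed checkpoint race, won by crossing the finish line before time runs out.
; On BeginPlay it binds to every BP_Checkpoint's dispatchers, separating the finish line from time-bonus checkpoints, then runs a start countdown.
; A single timer handle drives the time limit, re-armed with remaining time plus each bonus and cleared on a win.
; Countdown, start and win/lose feedback are only printed strings.
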(event `self.ReceiveBeginPlay`
  ;[1 1 0.4] Eventi
  (`|ExecutionSequence`
    (:`then_0`
      ;[1 1 1] Identifica i blocchi BP_Checkpoint e associa il ricevitore di messaggio
      (bind _outactors (`GameplayStatics.GetAllActorsOfClass` "/Game/GPCastle/CheckPoints/BP_Checkpoint.BP_Checkpoint_C"))
      (for _array_element _outactors
        (if (`/Game/GPCastle/CheckPoints/BP_Checkpoint.IsFinishLine` _array_element)
          ;[1 1 1] Associa dispacer finish line
          (add `/Game/GPCastle/CheckPoints/BP_Checkpoint.OnCheckpointCrossed` _array_element (`|CreateDelegate` :!event `Win_CrossTheFinishLine`))
          (else
            ;[1 1 1] Associa dispaccer aggungi tempo
            (add `/Game/GPCastle/CheckPoints/BP_Checkpoint.OnCheckpointCrossedWithTime` _array_element (`|CreateDelegate` :!event `CrossedACheckpoint`))))))
    (:`then_1`
      (`self.StartCountdown`))))

(event `StartCountdown`
  ;[1 1 0.4] Eventi
  (`KismetSystemLibrary.PrintString` "Start Countdown" true true (struct :`G` 0.66 :`B` 1.0 :`A` 1.0) 10.0)
  (`KismetSystemLibrary.Delay` (`self.StartCountdownDuration`))
  (`self.GameStart`))

(event `GameStart`
  ;[1 1 0.4] Eventi
  (`KismetSystemLibrary.PrintString` "Game has started")
  (bind _returnvalue (`KismetSystemLibrary.K2_SetTimerDelegate` (delegate `Lose_OutOfTime`) (`self.StartTimerDuration`)))
  (set `self.TimeRemainingTimer` _returnvalue))

(event `Lose_OutOfTime`
  ;[1 1 0.4] Eventi
  (`self.GameFinish` false))

(event `GameFinish`
  (params (Win :type Boolean))
  ;[1 1 0.4] Eventi
  (`KismetSystemLibrary.PrintString` (`KismetMathLibrary.SelectString` "You Win" "You Lose" Win)))

(event `Win_CrossTheFinishLine`
  ;[1 1 0.4] Eventi
  (`KismetSystemLibrary.K2_ClearAndInvalidateTimerHandle` (`self.TimeRemainingTimer`))
  (`self.GameFinish` true))

(event `CrossedACheckpoint`
  (params (TimeToAdd :type Integer))
  ;[1 1 0.4] Eventi
  (`self.AddTimeToTimer` TimeToAdd))

(fn `AddTimeToTimer`
  (params (TimeToAdd :type Integer))
  (bind _returnvalue (`KismetSystemLibrary.K2_SetTimerDelegate` (`|CreateDelegate` :!event `Lose_OutOfTime`) (+ TimeToAdd (`KismetSystemLibrary.K2_GetTimerRemainingTimeHandle` (`self.TimeRemainingTimer`)))))
  (set `self.TimeRemainingTimer` _returnvalue))

(fn `UserConstructionScript`)