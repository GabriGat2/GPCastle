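; BP_BarrierTool is an editor placement tool that builds a straight barrier of repeated meshes toward an EndPoint.
; The construction script assigns MeshToSpawn and Scale to an instanced static mesh component, then derives the instance count from the scale-adjusted EndPoint distance and mesh Width.
; Instances are spaced by Width along the look-at direction, rotated to match and shifted back by EndPointOffset widths.
; The Event Graph holds no active logic.
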(fn `UserConstructionScript`
  (locals (NewLocalVar :type "Transform Structure"))
  (bind _width (`self.Width`))
  (bind _returnvalue (`KismetMathLibrary.FindLookAtRotation` (0.0 0.0 0.0) (`self.EndPoint`)))
  ;[1 1 1] Seleziona la static mesh
  (`StaticMeshComponent.SetStaticMesh` (`self.InstancedStaticMesh`) (`self.MeshToSpawn`))
  ;[1 1 1] Scala la static mesh
  (`SceneComponent.SetRelativeScale3D` (`self.InstancedStaticMesh`) (`self.Scale`))
  ;[1 1 1] Loop generazione istanze delle mesh
  (for _index (range (+ (`KismetMathLibrary.FFloor` (/ (`KismetMathLibrary.VSize` (/ (`self.EndPoint`) (`self.Scale`))) (`self.Width`))) 1))
    ;;[1 1 1] Instanzia la mesh
    (`InstancedStaticMeshComponent.AddInstance` (`self.InstancedStaticMesh`) (`KismetMathLibrary.MakeTransform` (* (- (* _index _width) (* _width (`self.EndPointOffset`))) (`KismetMathLibrary.GetForwardVector` _returnvalue)) _returnvalue) false)))