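; Construction-time barrier placement tool that lays copies of a chosen static mesh along an editable spline.
; The construction script assigns MeshToSpawn to an instanced static mesh component, then adds one local-space instance at each spline point.
; Each instance is oriented along that point's tangent and uses a shared Scale, so spline point count sets mesh count, with no runtime logic.
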(fn `UserConstructionScript`
  ;[1 1 1] Seleziona la static mesh
  (`StaticMeshComponent.SetStaticMesh` (`self.InstancedStaticMesh`) (`self.MeshToSpawn`))
  ;[1 1 1] Loop generazione istanze delle mesh
  (for _index (range (`SplineComponent.GetNumberOfSplinePoints` (`self.Spline`)))
    (bind (_location _tangent) (`SplineComponent.GetLocationAndTangentAtSplinePoint` (`self.Spline`) _index "Local"))
    ;;[1 1 1] Istanzia la mesh
    (`InstancedStaticMeshComponent.AddInstance` (`self.InstancedStaticMesh`) (`KismetMathLibrary.MakeTransform` _location (`KismetMathLibrary.Conv_VectorToRotator` _tangent) (`self.Scale`)) false)))