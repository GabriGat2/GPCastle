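; Spline tool actor that lays a row of decals along an editable path on the surface below, built in the construction script.
; Each spline point is snapped vertically by a Visibility line trace within a threshold, plus a Z offset.
; Downward-projecting decal components are then added at scale-based intervals along the spline, following its yaw and roll, with optional skipping.
; Instanced mesh and text render logic remains unconnected and never runs.
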(fn `UserConstructionScript`
  (locals (Index :type Integer) (NewLocalVar :type "Vector Structure"))
  (bind _splinedecalplacer (`self.SplineDecalPlacer`))
  (bind _decalsnapthreeshold (`self.DecalSnapThreeshold`))
  (bind _decalscale (`self.DecalScale`))
  (`|ExecutionSequence`
    (:`then_0`
      ;[1 1 1] Inizializzazioni
      ;;[1 1 1] Determita i punti della spline
      (set `self.NumberSplinePoints` (`SplineComponent.GetNumberOfSplinePoints` (`self.SplineDecalPlacer`)))
      ;;[1 1 1] Azzera il contatore di punti della spline modicati
      (set `self.NumberSplinePointsChanged` 0))
    (:`then_1`
      ;[1 1 1] Sposta la coordinata Z del punto della spline sulla superficie
      (for _index (range (`self.NumberSplinePoints`))
        (bind _output_get (set `local.Index` _index))
        (bind (_returnvalue_x _returnvalue_y _returnvalue_z) (`KismetMathLibrary.BreakVector` (`SplineComponent.GetLocationAtSplinePoint` (`self.SplineDecalPlacer`) _output_get "World")))
        ;;[1 1 1] Raytracing per trovare il punto sul piano
        (bind (_outhit _returnvalue) (`KismetSystemLibrary.LineTraceSingle` :`Start` (`KismetMathLibrary.MakeVector` _returnvalue_x _returnvalue_y (+ _returnvalue_z _decalsnapthreeshold)) :`End` (`KismetMathLibrary.MakeVector` _returnvalue_x _returnvalue_y (- _returnvalue_z _decalsnapthreeshold)) :`TraceChannel` "TraceTypeQuery1" :`DrawTime` 2.0))
        ;;[1 1 1] Modifica la coordinata Z del punto della spline
        (if _returnvalue
          (set `self.NumberSplinePointsChanged` (+ (`self.NumberSplinePointsChanged`) 1))
          (`SplineComponent.SetLocationAtSplinePoint` (`self.SplineDecalPlacer`) (`local.Index`) (`KismetMathLibrary.MakeVector` _returnvalue_x _returnvalue_y (+ (.z (`.Location` (`GameplayStatics.BreakHitResult` _outhit))) (`self.DecalZOffset`))) "World" true))))
    (:`then_2`
      ;[1 1 1] Aggiunge le decal
      ;;[1 1 1] Calcola la dimensione scalata della decal
      (set `self.DecalSize` (* (* 512.0 (`self.DecalScale`)) (`self.DecalOffset`)))
      (for _index_2 (range (+ (`KismetMathLibrary.FTrunc` (`KismetMathLibrary.FClamp` (/ (`SplineComponent.GetSplineLength` (`self.SplineDecalPlacer`)) (`self.DecalSize`)) 0.0 1000.0)) 1))
        ;;[1 1 1] Aggiunge un componente decal
        (if (== (mod _index_2 (`self.SkipDecal`)) 0)
          (bind _returnvalue_2 (`AddComponent|NODE_AddDecalComponent-0` :`RelativeTransform` (`KismetMathLibrary.MakeTransform` (0.0 0.0 0.0) (struct :`Pitch` 90.0) (`KismetMathLibrary.MakeVector` (`self.ProjectionScale`) _decalscale _decalscale))))
          (bind _returnvalue_3 (* _index_2 (`self.DecalSize`)))
          (bind (_returnvalue_x_2 _returnvalue_y_2 _returnvalue_z_2) (`KismetMathLibrary.BreakVector` (`SplineComponent.GetLocationAtDistanceAlongSpline` _splinedecalplacer _returnvalue_3 "World")))
          (bind (_returnvalue_roll _returnvalue_pitch _returnvalue_yaw) (`KismetMathLibrary.BreakRotator` (`SplineComponent.GetRotationAtDistanceAlongSpline` _splinedecalplacer _returnvalue_3 "World")))
          ;;[1 1 1] Calcola la posizione della decal sulla spline
          (`SceneComponent.K2_SetWorldLocationAndRotation` _returnvalue_2 (`KismetMathLibrary.MakeVector` _returnvalue_x_2 _returnvalue_y_2 _returnvalue_z_2) (`KismetMathLibrary.MakeRotator` _returnvalue_roll 90.0 _returnvalue_yaw) false false)
          ;;[1 1 1] Aggiunge il materiale della decal
          (`DecalComponent.SetDecalMaterial` _returnvalue_2 (`self.DecalToPlace`)))))))