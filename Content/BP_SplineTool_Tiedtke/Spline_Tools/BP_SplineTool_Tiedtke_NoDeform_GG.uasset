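; Spline placement tool that tiles a static mesh along a spline as undeformed instances, built entirely in the construction script.
; Spacing comes from the mesh's scaled X bounds plus an offset, and the spline length divided by it sets the instance count.
; Each instance sits at its distance along the spline, oriented along the chord between points half a spacing behind and ahead.
; The actor's collision is toggled by a setting.
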(fn `Get Location At Index`
  (params (A :type Integer) (NewParam :type Integer))
  (returns (ReturnValue :type "Vector Structure"))
  (return (`SplineComponent.GetLocationAtDistanceAlongSpline` (`self.Spline`) (* A (`self.Spacing`)) "Local")))

(fn `GetRotationAtIndex`
  (params (A :type Integer))
  (returns (ReturnValue :type "Rotator Structure"))
  (bind _spline (`self.Spline`))
  (bind _spacing (`self.Spacing`))
  (bind _returnvalue (* A _spacing))
  (bind _returnvalue_2 (/ _spacing 2.0))
  (return (`KismetMathLibrary.MakeRotFromX` (- (`SplineComponent.GetLocationAtDistanceAlongSpline` _spline (+ _returnvalue _returnvalue_2) "Local") (`SplineComponent.GetLocationAtDistanceAlongSpline` _spline (- _returnvalue _returnvalue_2) "Local")))))

(fn `UserConstructionScript`
  (locals (`Number Of Instances` :type Integer :default 0))
  (bind _scale_x (`KismetMathLibrary.BreakVector` (`self.Scale`)))
  (bind (_min _max) (break `Box` (`StaticMesh.GetBoundingBox` (`self.Spline Mesh`))))
  (`StaticMeshComponent.SetStaticMesh` (`self.InstancedStaticMesh`) (`self.Spline Mesh`))
  (`self.SetActorEnableCollision` (`self.Collision?`))
  ;[1 1 1] Tile Next Mesh
  (bind _output_get (set `self.Spacing` (+ (* (.x (- _max _min)) _scale_x) (`self.Spline Mesh Offset`))))
  (bind _output_get_2 (set `local.Number Of Instances` (`KismetMathLibrary.FFloor` (/ (`SplineComponent.GetSplineLength` (`self.Spline`)) _output_get))))
  (for _index (range (+ _output_get_2 1))
    (`InstancedStaticMeshComponent.AddInstance` (`self.InstancedStaticMesh`) (`KismetMathLibrary.MakeTransform` (`self.Get Location At Index` _index) (`self.GetRotationAtIndex` _index) (`self.Scale`)) false)))